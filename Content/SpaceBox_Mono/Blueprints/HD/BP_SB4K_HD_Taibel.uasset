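; BP_SB4K_HD_Taibel is a space skybox actor that shows the HD Taibel background from the SpaceBox Mono content.
; Its construction script sets the actor scale from a Scale variable and assigns a dedicated material to each of the six face components: Up, Down, Left, Right, Front and Back.
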(fn `UserConstructionScript`
  (`self.SetActorScale3D` (`self.Scale`))
  (`PrimitiveComponent.SetMaterial` (`self.Up`) 0 "/Game/SpaceBox_Mono/Materials/HD/Taibel/Mat_HD_Taibel_Up.Mat_HD_Taibel_Up")
  (`PrimitiveComponent.SetMaterial` (`self.Right`) 0 "/Game/SpaceBox_Mono/Materials/HD/Taibel/Mat_HD_Taibel_Right.Mat_HD_Taibel_Right")
  (`PrimitiveComponent.SetMaterial` (`self.Left`) 0 "/Game/SpaceBox_Mono/Materials/HD/Taibel/Mat_HD_Taibel_Left.Mat_HD_Taibel_Left")
  (`PrimitiveComponent.SetMaterial` (`self.Front`) 0 "/Game/SpaceBox_Mono/Materials/HD/Taibel/Mat_HD_Taibel_Front.Mat_HD_Taibel_Front")
  (`PrimitiveComponent.SetMaterial` (`self.Down`) 0 "/Game/SpaceBox_Mono/Materials/HD/Taibel/Mat_HD_Taibel_Down.Mat_HD_Taibel_Down")
  (`PrimitiveComponent.SetMaterial` (`self.Back`) 0 "/Game/SpaceBox_Mono/Materials/HD/Taibel/Mat_HD_Taibel_Back.Mat_HD_Taibel_Back"))