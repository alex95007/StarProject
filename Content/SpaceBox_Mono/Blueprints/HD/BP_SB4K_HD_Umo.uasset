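; BP_SB4K_HD_Umo is a space skybox actor for the HD Umo set in SpaceBox_Mono, built from six face components.
; Its construction script sets the actor's 3D scale from the Scale variable.
; It then assigns the matching Umo material to the first slot of each face: Up, Down, Left, Right, Front and Back.
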(fn `UserConstructionScript`
  (`self.SetActorScale3D` (`self.Scale`))
  (`PrimitiveComponent.SetMaterial` (`self.Up`) 0 "/Game/SpaceBox_Mono/Materials/HD/Umo/Mat_HD_Umo_Up.Mat_HD_Umo_Up")
  (`PrimitiveComponent.SetMaterial` (`self.Right`) 0 "/Game/SpaceBox_Mono/Materials/HD/Umo/Mat_HD_Umo_Right.Mat_HD_Umo_Right")
  (`PrimitiveComponent.SetMaterial` (`self.Left`) 0 "/Game/SpaceBox_Mono/Materials/HD/Umo/Mat_HD_Umo_Left.Mat_HD_Umo_Left")
  (`PrimitiveComponent.SetMaterial` (`self.Front`) 0 "/Game/SpaceBox_Mono/Materials/HD/Umo/Mat_HD_Umo_Front.Mat_HD_Umo_Front")
  (`PrimitiveComponent.SetMaterial` (`self.Down`) 0 "/Game/SpaceBox_Mono/Materials/HD/Umo/Mat_HD_Umo_Down.Mat_HD_Umo_Down")
  (`PrimitiveComponent.SetMaterial` (`self.Back`) 0 "/Game/SpaceBox_Mono/Materials/HD/Umo/Mat_HD_Umo_Back.Mat_HD_Umo_Back"))