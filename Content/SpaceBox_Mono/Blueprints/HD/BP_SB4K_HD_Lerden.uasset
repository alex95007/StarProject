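; BP_SB4K_HD_Lerden is a skybox actor, apparently the HD "Lerden" variant of the SpaceBox_Mono set, built from six face components.
; Its construction script sets the actor's scale from a Scale variable, then assigns the matching Lerden material to the Up, Down, Left, Right, Front and Back faces.
; The file contains no other logic, so all setup happens at construction.
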(fn `UserConstructionScript`
  (`self.SetActorScale3D` (`self.Scale`))
  (`PrimitiveComponent.SetMaterial` (`self.Up`) 0 "/Game/SpaceBox_Mono/Materials/HD/Lerden/Mat_HD_Lerden_Up.Mat_HD_Lerden_Up")
  (`PrimitiveComponent.SetMaterial` (`self.Right`) 0 "/Game/SpaceBox_Mono/Materials/HD/Lerden/Mat_HD_Lerden_Right.Mat_HD_Lerden_Right")
  (`PrimitiveComponent.SetMaterial` (`self.Left`) 0 "/Game/SpaceBox_Mono/Materials/HD/Lerden/Mat_HD_Lerden_Left.Mat_HD_Lerden_Left")
  (`PrimitiveComponent.SetMaterial` (`self.Front`) 0 "/Game/SpaceBox_Mono/Materials/HD/Lerden/Mat_HD_Lerden_Front.Mat_HD_Lerden_Front")
  (`PrimitiveComponent.SetMaterial` (`self.Down`) 0 "/Game/SpaceBox_Mono/Materials/HD/Lerden/Mat_HD_Lerden_Down.Mat_HD_Lerden_Down")
  (`PrimitiveComponent.SetMaterial` (`self.Back`) 0 "/Game/SpaceBox_Mono/Materials/HD/Lerden/Mat_HD_Lerden_Back.Mat_HD_Lerden_Back"))