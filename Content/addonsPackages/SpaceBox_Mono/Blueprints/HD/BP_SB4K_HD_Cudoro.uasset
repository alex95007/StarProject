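; BP_SB4K_HD_Cudoro is a space skybox actor from the SpaceBox Mono addon, showing the HD Cudoro backdrop.
; Its construction script sets the actor's 3D scale from a Scale variable.
; It then assigns a dedicated Cudoro material to each of the six face components (Up, Down, Left, Right, Front, Back), with no other logic.
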(fn `UserConstructionScript`
  (`self.SetActorScale3D` (`self.Scale`))
  (`PrimitiveComponent.SetMaterial` (`self.Up`) 0 "/Game/addonsPackages/SpaceBox_Mono/Materials/HD/Cudoro/Mat_HD_Cudoro_Up.Mat_HD_Cudoro_Up")
  (`PrimitiveComponent.SetMaterial` (`self.Right`) 0 "/Game/addonsPackages/SpaceBox_Mono/Materials/HD/Cudoro/Mat_HD_Cudoro_Right.Mat_HD_Cudoro_Right")
  (`PrimitiveComponent.SetMaterial` (`self.Left`) 0 "/Game/addonsPackages/SpaceBox_Mono/Materials/HD/Cudoro/Mat_HD_Cudoro_Left.Mat_HD_Cudoro_Left")
  (`PrimitiveComponent.SetMaterial` (`self.Front`) 0 "/Game/addonsPackages/SpaceBox_Mono/Materials/HD/Cudoro/Mat_HD_Cudoro_Front.Mat_HD_Cudoro_Front")
  (`PrimitiveComponent.SetMaterial` (`self.Down`) 0 "/Game/addonsPackages/SpaceBox_Mono/Materials/HD/Cudoro/Mat_HD_Cudoro_Down.Mat_HD_Cudoro_Down")
  (`PrimitiveComponent.SetMaterial` (`self.Back`) 0 "/Game/addonsPackages/SpaceBox_Mono/Materials/HD/Cudoro/Mat_HD_Cudoro_Back.Mat_HD_Cudoro_Back"))