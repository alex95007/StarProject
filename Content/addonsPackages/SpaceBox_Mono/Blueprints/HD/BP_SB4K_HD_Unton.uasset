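; BP_SB4K_HD_Unton is a space box actor from the SpaceBox_Mono addon that displays the HD "Unton" backdrop on six faces.
; Its construction script sets the actor's scale from the Scale variable, then assigns a dedicated Unton material to each of the Up, Down, Left, Right, Front and Back components.
; The file contains no logic beyond this construction-time setup.
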(fn `UserConstructionScript`
  (`self.SetActorScale3D` (`self.Scale`))
  (`PrimitiveComponent.SetMaterial` (`self.Up`) 0 "/Game/addonsPackages/SpaceBox_Mono/Materials/HD/Unton/Mat_HD_Unton_Up.Mat_HD_Unton_Up")
  (`PrimitiveComponent.SetMaterial` (`self.Right`) 0 "/Game/addonsPackages/SpaceBox_Mono/Materials/HD/Unton/Mat_HD_Unton_Right.Mat_HD_Unton_Right")
  (`PrimitiveComponent.SetMaterial` (`self.Left`) 0 "/Game/addonsPackages/SpaceBox_Mono/Materials/HD/Unton/Mat_HD_Unton_Left.Mat_HD_Unton_Left")
  (`PrimitiveComponent.SetMaterial` (`self.Front`) 0 "/Game/addonsPackages/SpaceBox_Mono/Materials/HD/Unton/Mat_HD_Unton_Front.Mat_HD_Unton_Front")
  (`PrimitiveComponent.SetMaterial` (`self.Down`) 0 "/Game/addonsPackages/SpaceBox_Mono/Materials/HD/Unton/Mat_HD_Unton_Down.Mat_HD_Unton_Down")
  (`PrimitiveComponent.SetMaterial` (`self.Back`) 0 "/Game/addonsPackages/SpaceBox_Mono/Materials/HD/Unton/Mat_HD_Unton_Back.Mat_HD_Unton_Back"))