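; BP_SB4K_HD_Tairan is a space skybox actor from the SpaceBox_Mono add-on that shows the HD Tairan backdrop.
; Its construction script scales the actor by the Scale variable.
; It then assigns a dedicated Tairan material to each of the six face components (Up, Down, Left, Right, Front, Back).
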(fn `UserConstructionScript`
  (`self.SetActorScale3D` (`self.Scale`))
  (`PrimitiveComponent.SetMaterial` (`self.Up`) 0 "/Game/addonsPackages/SpaceBox_Mono/Materials/HD/Tairan/Mat_HD_Tairan_Up.Mat_HD_Tairan_Up")
  (`PrimitiveComponent.SetMaterial` (`self.Right`) 0 "/Game/addonsPackages/SpaceBox_Mono/Materials/HD/Tairan/Mat_HD_Tairan_Right.Mat_HD_Tairan_Right")
  (`PrimitiveComponent.SetMaterial` (`self.Left`) 0 "/Game/addonsPackages/SpaceBox_Mono/Materials/HD/Tairan/Mat_HD_Tairan_Left.Mat_HD_Tairan_Left")
  (`PrimitiveComponent.SetMaterial` (`self.Front`) 0 "/Game/addonsPackages/SpaceBox_Mono/Materials/HD/Tairan/Mat_HD_Tairan_Front.Mat_HD_Tairan_Front")
  (`PrimitiveComponent.SetMaterial` (`self.Down`) 0 "/Game/addonsPackages/SpaceBox_Mono/Materials/HD/Tairan/Mat_HD_Tairan_Down.Mat_HD_Tairan_Down")
  (`PrimitiveComponent.SetMaterial` (`self.Back`) 0 "/Game/addonsPackages/SpaceBox_Mono/Materials/HD/Tairan/Mat_HD_Tairan_Back.Mat_HD_Tairan_Back"))