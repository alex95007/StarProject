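; BP_SB4K_HD_Lyekal is the HD "Lyekal" space skybox actor from the SpaceBox_Mono addon package.
; Its construction script sets the actor's scale from a Scale variable, then assigns a separate material to each of six face components (Up, Down, Left, Right, Front, Back) to form the surrounding cube.
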(fn `UserConstructionScript`
  (`self.SetActorScale3D` (`self.Scale`))
  (`PrimitiveComponent.SetMaterial` (`self.Up`) 0 "/Game/addonsPackages/SpaceBox_Mono/Materials/HD/Lyekal/Mat_HD_Lyekal_Up.Mat_HD_Lyekal_Up")
  (`PrimitiveComponent.SetMaterial` (`self.Right`) 0 "/Game/addonsPackages/SpaceBox_Mono/Materials/HD/Lyekal/Mat_HD_Lyekal_Right.Mat_HD_Lyekal_Right")
  (`PrimitiveComponent.SetMaterial` (`self.Left`) 0 "/Game/addonsPackages/SpaceBox_Mono/Materials/HD/Lyekal/Mat_HD_Lyekal_Left.Mat_HD_Lyekal_Left")
  (`PrimitiveComponent.SetMaterial` (`self.Front`) 0 "/Game/addonsPackages/SpaceBox_Mono/Materials/HD/Lyekal/Mat_HD_Lyekal_Front.Mat_HD_Lyekal_Front")
  (`PrimitiveComponent.SetMaterial` (`self.Down`) 0 "/Game/addonsPackages/SpaceBox_Mono/Materials/HD/Lyekal/Mat_HD_Lyekal_Down.Mat_HD_Lyekal_Down")
  (`PrimitiveComponent.SetMaterial` (`self.Back`) 0 "/Game/addonsPackages/SpaceBox_Mono/Materials/HD/Lyekal/Mat_HD_Lyekal_Back.Mat_HD_Lyekal_Back"))